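; BP_PaperLevelSequenceActor is an actor that cycles through the red, blue and green paper level sequences in an endless timed loop.
; On BeginPlay it creates and stores a player per sequence, then starts PlayPaperSequence.
; That self-calling event waits on a fixed delay, plays the sequence selected by CurrentSequenceNum and advances the index.
; Each pass creates a fresh player, so the stored Red, Blue and Green players are never played.
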(event `self.ReceiveBeginPlay`
  (bind (_outactor _returnvalue) (`LevelSequencePlayer.CreateLevelSequencePlayer` "/Game/_Sparta/LevelSequence/LS_Paper_Red.LS_Paper_Red"))
  (set `self.Red` _returnvalue)
  (bind (_outactor_2 _returnvalue_2) (`LevelSequencePlayer.CreateLevelSequencePlayer` "/Game/_Sparta/LevelSequence/LS_Paper_Blue.LS_Paper_Blue"))
  (set `self.Blue` _returnvalue_2)
  (bind (_outactor_3 _returnvalue_3) (`LevelSequencePlayer.CreateLevelSequencePlayer` "/Game/_Sparta/LevelSequence/LS_Paper_Green.LS_Paper_Green"))
  (set `self.Green` _returnvalue_3)
  (`self.PlayPaperSequence`))

(event `PlayPaperSequence`
  (`KismetSystemLibrary.Delay` 20.0)
  (switch `int` (`self.CurrentSequenceNum`)
    (:`0`
      (bind (_outactor _returnvalue) (`LevelSequencePlayer.CreateLevelSequencePlayer` "/Game/_Sparta/LevelSequence/LS_Paper_Red.LS_Paper_Red"))
      (`MovieSceneSequencePlayer.Play` _returnvalue)
      (set `self.CurrentSequenceNum` 1)
      (`self.PlayPaperSequence`))
    (:`1`
      (bind (_outactor_2 _returnvalue_2) (`LevelSequencePlayer.CreateLevelSequencePlayer` "/Game/_Sparta/LevelSequence/LS_Paper_Blue.LS_Paper_Blue"))
      (`MovieSceneSequencePlayer.Play` _returnvalue_2)
      (set `self.CurrentSequenceNum` 2)
      (`self.PlayPaperSequence`))
    (:`2`
      (bind (_outactor_3 _returnvalue_3) (`LevelSequencePlayer.CreateLevelSequencePlayer` "/Game/_Sparta/LevelSequence/LS_Paper_Green.LS_Paper_Green"))
      (`MovieSceneSequencePlayer.Play` _returnvalue_3)
      (set `self.CurrentSequenceNum` 0)
      (`self.PlayPaperSequence`))))

(fn `UserConstructionScript`)